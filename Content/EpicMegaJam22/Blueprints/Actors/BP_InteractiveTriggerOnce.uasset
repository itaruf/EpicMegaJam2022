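; BP_InteractiveTriggerOnce is a trigger actor that fires an interaction when the BP_TwoWorldsCharacter player overlaps it.
; On begin overlap it skips if it is unusable or is a one-time trigger that already fired.
; Otherwise it marks itself triggered and calls CallEDIOnInteractOnceTriggered with itself, apparently an event dispatcher broadcast.
; End overlap only casts to the character and does nothing further.
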(event Collision|EventActorBeginOverlap
  (params (OtherActor :type Actor%20Object%20Reference))
  (if (not (or (and (Variables|Default|GetIsOneTimeTrigger) (Variables|Default|GetHasBeenTriggered)) (not (Variables|Default|GetIsUsable))))
    (Utilities|Casting|CastToBP_TwoWorldsCharacter OtherActor)
    (Variables|Default|SetHasBeenTriggered true)
    (Default|CallEDIonInteractOnceTriggered self)))

(event Collision|EventActorEndOverlap
  (params (OtherActor :type Actor%20Object%20Reference))
  (Utilities|Casting|CastToBP_TwoWorldsCharacter OtherActor))

(fn ConstructionScript)