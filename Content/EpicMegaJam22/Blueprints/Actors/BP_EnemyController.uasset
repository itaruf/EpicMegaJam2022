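; AI controller for an exploding enemy that runs BT_Enemy with the player as Target and the enemy's Start as home.
; Fast looping timers drive distance checks for trigger range, explosion range and leash, with two timers swapping to flag returning home and arrival.
; Reaching explosion range fires an exploding dispatcher that flags the blackboard and stops that check.
; KABOOM kills a player overlapping the explosion radius; movement-mode switching logic is left unconnected.
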(event Custom|Check%20Explosion%20Range
  (if (<= (Math|Vector|Distance(Vector) (Transformation|GetActorLocation (Variables|Owner|GetBP%20Enemy)) (Transformation|GetActorLocation (Game|Player|GetPlayerPawn 0))) (Variables|/Game/EpicMegaJam22/Blueprints/Actors/BP_Enemy.BP_Enemy_C|GetExplosionRange (Variables|Owner|GetBP%20Enemy)))
    (Default|CallEDIonExploding)))

(event Custom|On%20Exploding
  (Utilities|FlowControl|Sequence
    (:then_0
      (AI|Components|Blackboard|SetValueasBool (Variables|Default|GetBlackboard) (Utilities|Name|MakeLiteralName "InExplosionRange") true))
    (:then_1
      (Utilities|Time|ClearandInvalidateTimerbyHandle (Variables|Timer|GetCheck%20Exp%20Range%20Timer)))))

(event Custom|Has%20Back%20to%20Start
  (bind _bp_enemy (Variables|Owner|GetBP%20Enemy))
  (if (<= (Math|Vector|Distance(Vector) (Variables|/Game/EpicMegaJam22/Blueprints/Actors/BP_Enemy.BP_Enemy_C|GetStart _bp_enemy) (Transformation|GetActorLocation _bp_enemy)) 5e+02)
    (AI|Components|Blackboard|SetValueasBool (Variables|Default|GetBlackboard) (Utilities|Name|MakeLiteralName "ShouldBackToStart") false)
    (Utilities|Time|ClearandInvalidateTimerbyHandle (Variables|Timer|GetHas%20Backed%20to%20Start%20Timer))
    (bind _returnvalue (Utilities|Time|SetTimerbyEvent (EventDispatchers|CreateEvent :!event Custom|Should%20Back%20To%20Start) 0.01 true))
    (Variables|Timer|SetShould%20Back%20to%20Start%20Timer _returnvalue)))

(event Custom|Should%20Back%20To%20Start
  (bind _bp_enemy (Variables|Owner|GetBP%20Enemy))
  (if (>= (Math|Vector|Distance(Vector) (Transformation|GetActorLocation _bp_enemy) (Variables|/Game/EpicMegaJam22/Blueprints/Actors/BP_Enemy.BP_Enemy_C|GetStart _bp_enemy)) (Variables|Range|GetMaxRange))
    (AI|Components|Blackboard|SetValueasBool (Variables|Default|GetBlackboard) (Utilities|Name|MakeLiteralName "ShouldBackToStart") true)
    (Utilities|Time|ClearandInvalidateTimerbyHandle (Variables|Timer|GetShould%20Back%20to%20Start%20Timer))
    (bind _returnvalue (Utilities|Time|SetTimerbyEvent (EventDispatchers|CreateEvent :!event Custom|Has%20Back%20to%20Start) 0.01 true))
    (Variables|Timer|SetHas%20Backed%20to%20Start%20Timer _returnvalue)))

(event Custom|KABOOM
  (bind _returnvalue (Game|Player|GetPlayerPawn 0))
  (if (Collision|IsOverlappingActor (Variables|/Game/EpicMegaJam22/Blueprints/Actors/BP_Enemy.BP_Enemy_C|GetExplosion%20Radius (Variables|Owner|GetBP%20Enemy)) _returnvalue :!class /Script/Engine.PrimitiveComponent)
    (bind _asbp_two_worlds_character (Utilities|Casting|CastToBP_TwoWorldsCharacter _returnvalue))
    (Default|Die(Explosion) _asbp_two_worlds_character)))

(event Custom|Is%20Target%20In%20Range
  (if (< (Math|Vector|Distance(Vector) (Transformation|GetActorLocation (Variables|Owner|GetBP%20Enemy)) (Transformation|GetActorLocation (Game|Player|GetPlayerPawn 0))) (Variables|/Game/EpicMegaJam22/Blueprints/Actors/BP_Enemy.BP_Enemy_C|GetTargetTriggerRange (Variables|Owner|GetBP%20Enemy)))
    (AI|Components|Blackboard|SetValueasBool (Variables|Default|GetBlackboard) (Utilities|Name|MakeLiteralName "ShouldBackToStart") false)
    (else
      (AI|Components|Blackboard|SetValueasBool (Variables|Default|GetBlackboard) (Utilities|Name|MakeLiteralName "ShouldBackToStart") true))))

(event EventBeginPlay
  (Utilities|FlowControl|Sequence
    (:then_0
      (bind _asbp_enemy (Utilities|Casting|CastToBP_Enemy (Pawn|GetControlledPawn)))
      (bind _output_get (Variables|Owner|SetBP%20Enemy _asbp_enemy)))
    (:then_1
      (AI|RunBehaviorTree "/Game/EpicMegaJam22/Blueprints/AI/BT_Enemy.BT_Enemy")
      (AI|Components|Blackboard|SetValueasObject (Variables|Default|GetBlackboard) (Utilities|Name|MakeLiteralName "Target") (Game|Player|GetPlayerPawn 0))
      (AI|Components|Blackboard|SetValueasVector (Variables|Default|GetBlackboard) (Utilities|Name|MakeLiteralName "Start") (Variables|/Game/EpicMegaJam22/Blueprints/Actors/BP_Enemy.BP_Enemy_C|GetStart (Variables|Owner|GetBP%20Enemy))))
    (:then_2
      (bind _returnvalue (Utilities|Time|SetTimerbyEvent (EventDispatchers|CreateEvent :!event Custom|Check%20Explosion%20Range) 0.01 true))
      (Variables|Timer|SetCheck%20Exp%20Range%20Timer _returnvalue)
      (bind _returnvalue_2 (Utilities|Time|SetTimerbyEvent (EventDispatchers|CreateEvent :!event Custom|Should%20Back%20To%20Start) 0.01 true))
      (Variables|Timer|SetShould%20Back%20to%20Start%20Timer _returnvalue_2)
      (EventDispatchers|BindEventtoEDIonExploding (EventDispatchers|CreateEvent :!event Custom|On%20Exploding))
      (Utilities|Time|SetTimerbyEvent (EventDispatchers|CreateEvent :!event Custom|Is%20Target%20In%20Range) 0.01 true))))

(event EventTick
  (params (DeltaSeconds :type Float%20%28single-precision%29))
  (AI|Components|Blackboard|SetValueasVector (Variables|Default|GetBlackboard) (Utilities|Name|MakeLiteralName "Start") (Variables|/Game/EpicMegaJam22/Blueprints/Actors/BP_Enemy.BP_Enemy_C|GetStart (Variables|Owner|GetBP%20Enemy))))

(fn ConstructionScript)