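; Player character for a two-worlds game, handling health, death (including by explosion), healing, sprinting, collectible pickups and the pause menu.
; Event dispatchers announce HUD setup, health, sprint, death and pickup changes.
; Sprinting raises walk and swim speeds, plays a camera shake and runs a looping timer until release.
; Tick eases the follow camera's pitch and height and adjusts view pitch limits to suit walking or swimming.
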(event Custom|On%20Sprinting
  (bind _shakesprint (Variables|Default|GetShakeSprint))
  ;[1 1 1] ON SPRINTING
  (CameraShakes|StartCameraShake _shakesprint (Variables|/Script/Engine.CameraShakeSourceComponent|GetCameraShake _shakesprint) 1.0 "CameraLocal" (Pawn|GetControlRotation :!class /Script/Engine.Pawn)))

(event Custom|HealPlayer
  (params (HealAmount :type Float%20%28double-precision%29))
  (bind _maxhealth (Variables|Default|GetMaxHealth))
  ;[1 1 1] Heal the player and notifies
  (bind _output_get (Variables|Default|SetCurrentHealth (Math|Float|Clamp(Float) (+ HealAmount (Variables|Default|GetCurrentHealth)) 0.0 _maxhealth)))
  (Default|CallEDIonHealthChange _output_get _maxhealth))

(event Custom|TakeDamage
  (params (DamageTaken :type Float%20%28double-precision%29))
  (bind _maxhealth (Variables|Default|GetMaxHealth))
  ;[1 1 1] Take damage and notifies
  (bind _output_get (Variables|Default|SetCurrentHealth (Math|Float|Clamp(Float) (- (Variables|Default|GetCurrentHealth) DamageTaken) 0.0 _maxhealth)))
  (Utilities|FlowControl|Sequence
    (:then_0
      (Default|CallEDIonHealthChange _output_get _maxhealth))
    (:then_1
      (if (and (<= _output_get 0.0) (not (Variables|Default|GetIsPlayedDead)))
        (CallFunction|Die)))))

(event Custom|AddCollectible
  ;[1 1 1] Add collectible
  (bind _result (Math|Integer|IncrementInt (Variables|Default|GetCollectedItems))
    (:%20%20
      (Audio|SpawnSoundatLocation "/Game/EpicMegaJam22/Audio/StartSelect_UI_set3_pure_warm_simple_quick_tonal_deaction.StartSelect_UI_set3_pure_warm_simple_quick_tonal_deaction" (Transformation|GetActorLocation) "0, 0, 0" 2.0 1.0 0.0 0 0)
      (Default|CallEDIonCollectedItem _result))))

(event Custom|Die
  ;[1 1 1] Handle death of the player
  (if (not (Variables|Default|GetIsPlayedDead))
    (Variables|Default|SetIsPlayedDead true)
    (Default|CallEDIonPlayerDeath)
    (Input|DisableInput (Variables|Default|GetPlayerController))))

(event Custom|Die%20%28Explosion%29
  (CallFunction|Die)
  (Default|CallEDIonPlayerDeath(Explosion)))

(event EventBeginPlay
  (bind _returnvalue (Game|GetPlayerController 0))
  ;[1 1 1] BEGIN PLAY
  (bind _asbp_two_worlds_hud (Utilities|Casting|CastToBP_TwoWorldsHud (HUD|GetHUD _returnvalue)))
  (Variables|Default|SetPlayerHudRef _asbp_two_worlds_hud)
  (Default|CallEDIonHudSet)
  (bind _aspc_two_worlds (Utilities|Casting|CastToPC_TwoWorlds _returnvalue))
  (Variables|Default|SetPlayerController _aspc_two_worlds))

(event EventTick
  (params (DeltaSeconds :type Float%20%28single-precision%29))
  (bind _returnvalue (Game|GetPlayerCameraManager 0))
  (bind _returnvalue_2 (Game|GetPlayerCameraManager 0))
  (bind _followcamera (Variables|Default|GetFollowCamera))
  (bind _followcamera_2 (Variables|Default|GetFollowCamera))
  (bind _followcamera_3 (Variables|Default|GetFollowCamera))
  (bind _followcamera_4 (Variables|Default|GetFollowCamera))
  (bind _relativerotation (Variables|/Script/Engine.SceneComponent|GetRelativeRotation _followcamera_4))
  (bind _relativerotation_2 (Variables|/Script/Engine.SceneComponent|GetRelativeRotation _followcamera))
  (bind _relativelocation (Variables|/Script/Engine.SceneComponent|GetRelativeLocation _followcamera_2))
  (bind _relativelocation_2 (Variables|/Script/Engine.SceneComponent|GetRelativeLocation _followcamera_3))
  (Variables|Default|SetDelta%20Seconds DeltaSeconds)
  (Utilities|FlowControl|Sequence
    (:then_0
      (switch Utilities|FlowControl|Switch|SwitchonEMovementMode (Variables|/Script/Engine.CharacterMovementComponent|GetMovementMode (Variables|Character|GetCharacterMovement))
        (:MOVE_Walking
          (Utilities|FlowControl|Sequence
            (:then_0
              (Transformation|SetRelativeRotation (Variables|Default|GetFollowCamera) (Math|Rotator|MakeRotator (.roll _relativerotation_2) (Math|Interpolation|FInterpTo (.pitch _relativerotation_2) 15.0 (Variables|Default|GetDelta%20Seconds) (Variables|Camera|GetCameraInterpSpeed)) (.yaw _relativerotation_2)) false false))
            (:then_1
              (Variables|/Script/Engine.PlayerCameraManager|SetViewPitchMin _returnvalue_2 (Math|Interpolation|FInterpTo (Variables|/Script/Engine.PlayerCameraManager|GetViewPitchMin (Game|GetPlayerCameraManager 0)) -89.9 (Variables|Default|GetDelta%20Seconds) (Variables|Camera|GetCameraInterpSpeed)))
              (Variables|/Script/Engine.PlayerCameraManager|SetViewPitchMax _returnvalue_2 1.2e+02))
            (:then_2
              (Transformation|SetRelativeLocation (Variables|Default|GetFollowCamera) (Math|Vector|MakeVector (.x _relativelocation) (.y _relativelocation) (Math|Interpolation|FInterpTo (.z _relativelocation) 9e+01 (Variables|Default|GetDelta%20Seconds) (Variables|Camera|GetCameraInterpSpeed))) false false))))
        (:MOVE_Swimming
          (Utilities|FlowControl|Sequence
            (:then_0
              (Transformation|SetRelativeRotation (Variables|Default|GetFollowCamera) (Math|Rotator|MakeRotator (.roll _relativerotation) (Math|Interpolation|FInterpTo (.pitch _relativerotation) -25.0 (Variables|Default|GetDelta%20Seconds) (Variables|Camera|GetCameraInterpSpeed)) (.yaw _relativerotation)) false false))
            (:then_1
              (Variables|/Script/Engine.PlayerCameraManager|SetViewPitchMin _returnvalue (Math|Interpolation|FInterpTo (Variables|/Script/Engine.PlayerCameraManager|GetViewPitchMin (Game|GetPlayerCameraManager 0)) -75.0 (Variables|Default|GetDelta%20Seconds) (Variables|Camera|GetCameraInterpSpeed)))
              (Variables|/Script/Engine.PlayerCameraManager|SetViewPitchMax _returnvalue 1e+02))
            (:then_2
              (Transformation|SetRelativeLocation (Variables|Default|GetFollowCamera) (Math|Vector|MakeVector (.x _relativelocation_2) (.y _relativelocation_2) (Math|Interpolation|FInterpTo (.z _relativelocation_2) 0.0 (Variables|Default|GetDelta%20Seconds) (Variables|Camera|GetCameraInterpSpeed))) false false))))))))

(event Input|ActionEvents|InputActionSprint
  (params (Key :type Key%20Structure :default "None"))
  (bind _charactermovement (Variables|Character|GetCharacterMovement))
  (bind _charactermovement_2 (Variables|Character|GetCharacterMovement))
  ;[1 1 1] SPRINT
  (:Pressed
    (Variables|/Script/Engine.CharacterMovementComponent|SetMaxWalkSpeed _charactermovement_2 (Variables|Movement|GetSprintSpeed))
    (Variables|/Script/Engine.CharacterMovementComponent|SetMaxSwimSpeed _charactermovement_2 (Variables|Movement|GetSprintSpeed))
    (Default|CallEDIonSprint)
    (if (not (Utilities|Time|IsTimerActivebyHandle (Variables|Default|GetSprintTimer)))
      (bind _returnvalue (Utilities|Time|SetTimerbyEvent (EventDispatchers|CreateEvent :!event Custom|On%20Sprinting) 1.0 true))
      (Variables|Default|SetSprintTimer _returnvalue)
      (CallFunction|OnSprinting)))
  (:Released
    (Variables|/Script/Engine.CharacterMovementComponent|SetMaxWalkSpeed _charactermovement (Variables|Movement|GetWalkSpeed))
    (Variables|/Script/Engine.CharacterMovementComponent|SetMaxSwimSpeed _charactermovement (Variables|Movement|GetWalkSpeed))
    (Default|CallEDIonUnsprint)
    (Utilities|Time|ClearandInvalidateTimerbyHandle (Variables|Default|GetSprintTimer))))

(event Input|ActionEvents|InputActionPause
  (params (Key :type Key%20Structure :default "None"))
  (bind _playerhudref (Variables|Default|GetPlayerHudRef))
  (bind _pausewidget (Variables|/Game/EpicMegaJam22/Blueprints/BP_TwoWorldsHud.BP_TwoWorldsHud_C|GetPauseWidget _playerhudref))
  ;[1 1 1] PAUSE MENU
  (:Pressed
    (if (Game|IsGamePaused)
      (Default|RemoveWidget _playerhudref _pausewidget false)
      (Utilities|Time|SetGlobalTimeDilation 1.0)
      (Game|SetGamePaused false)
      (else
        (Default|AddWidget _playerhudref _pausewidget true)
        (Utilities|Time|SetGlobalTimeDilation 0.0)
        (Game|SetGamePaused true)))))

(fn ConstructionScript
  (|CallParentFunction))