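; Moving platform actor that shifts by per-trigger offsets from a map, allowing only destinations found in GridPos.
; OnTriggerOnce locks out re-entry, disables the used trigger, re-enables the others and drives a delayed timeline move.
; BeginPlay binds a valid toggle trigger and starts a timeline move; ToggleMoving alternately stops and resumes a timeline.
; Resetposition restores the starting location, but its binding, the map-trigger bindings and starting-position capture sit in unconnected nodes.
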(event Custom|OnTriggerOnce
  (params (Trigger :type BP%20Interactive%20Trigger%20Once%20Object%20Reference))
  (bind _associatedtrigger (Variables|Default|GetAssociatedTrigger))
  (bind (_value _returnvalue) (Utilities|Map|Find _associatedtrigger Trigger))
  (if (and (not (Variables|Default|GetIsAlreadyUsed)) _returnvalue)
    (Variables|Default|SetIsAlreadyUsed true)
    ;[1 1 1] Setting the current trigger to be disabled
    (bind _keys (Utilities|Map|Keys (Variables|Default|GetAssociatedTrigger)))
    (for _array_element _keys
      (if (== _array_element Trigger)
        (Variables|/Game/EpicMegaJam22/Blueprints/Actors/BP_InteractiveTriggerOnce.BP_InteractiveTriggerOnce_C|SetIsUsable _array_element false)
        (bind _output_get (Variables|Default|SetVelocityImpulse _value))
        (if (.ReturnValue (Utilities|Map|Find (Variables|Default|GetGridPos) (+ _output_get (Transformation|GetWorldLocation (Variables|Default|GetPlateformStaticMesh)))))
          (Variables|Default|SetStartLocation (Transformation|GetWorldLocation (Variables|Default|GetPlateformStaticMesh)))
          (Utilities|FlowControl|Delay (Variables|Default|GetStartDelay))
          (Components|Timeline|SetPlayRate (Variables|Default|GetMove) (Variables|Default|GetSpeed))
          (bind _newtrack_0 (Timeline|Timeline_0 PlayFromStart)
            (:Update
              (Transformation|SetWorldLocation (Variables|Default|GetPlateformStaticMesh) (+ (Variables|Default|GetStartLocation) (* _newtrack_0 (Variables|Default|GetVelocityImpulse))) false false))
            (:Finished
              (Variables|Default|SetIsAlreadyUsed false :!label _label)))
          (else
            (goto _label)))
        (else
          (Variables|/Game/EpicMegaJam22/Blueprints/Actors/BP_InteractiveTriggerOnce.BP_InteractiveTriggerOnce_C|SetIsUsable _array_element true))))))

(event Custom|Resetposition
  (bind _keys (Utilities|Map|Keys (Variables|Default|GetAssociatedTrigger)))
  (for _array_element _keys
    (Variables|/Game/EpicMegaJam22/Blueprints/Actors/BP_InteractiveTriggerOnce.BP_InteractiveTriggerOnce_C|SetIsUsable _array_element false))
  (Timeline|Reset PlayFromStart
    (:Update
      (Transformation|SetWorldLocation (Variables|Default|GetPlateformStaticMesh) (Variables|Default|GetStartingPos) false false)
      (bind _keys_2 (Utilities|Map|Keys (Variables|Default|GetAssociatedTrigger)))
      (for _array_element_2 _keys_2
        (Variables|/Game/EpicMegaJam22/Blueprints/Actors/BP_InteractiveTriggerOnce.BP_InteractiveTriggerOnce_C|SetIsUsable _array_element_2 true)))))

(event Custom|ToggleMoving
  (params (Trigger :type BP%20Interactive%20Trigger%20Once%20Object%20Reference))
  (Utilities|FlowControl|FlipFlop
    (:A
      (Audio|Components|Audio|Stop (Variables|Default|GetTimeline_1)))
    (:B
      (Audio|Components|Audio|Play (Variables|Default|GetTimeline_1)))))

(event EventBeginPlay
  (bind _togglemovementtrigger (Variables|Default|GetToggleMovementTrigger)
    (:then
      (EventDispatchers|BindEventtoEDIonInteractOnceTriggered _togglemovementtrigger (EventDispatchers|CreateEvent :!event Custom|ToggleMoving))
      (Variables|Default|SetStartLocation (Transformation|GetWorldLocation (Variables|Default|GetPlateformStaticMesh)))
      (Utilities|FlowControl|Delay (Variables|Default|GetStartDelay))
      (Components|Timeline|SetPlayRate (Variables|Default|GetMove) (Variables|Default|GetSpeed))
      (bind _newtrack_0 (Timeline|Timeline_1 PlayFromStart)
        (:Update
          (Transformation|SetWorldLocation (Variables|Default|GetPlateformStaticMesh) (+ (Variables|Default|GetStartLocation) (* _newtrack_0 (Variables|Default|GetVelocityImpulse))) false false))))
    (:else)))

(fn ConstructionScript
  (|CallParentFunction))