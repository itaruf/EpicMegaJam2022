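; BP_MovingBox is a moving platform actor that shifts its static mesh along a timeline curve.
; On BeginPlay it records the mesh's world location, waits for a start delay, then plays the Move timeline at a configurable speed.
; Each update sets the mesh to that start location plus the curve value scaled by a velocity impulse, without sweeping.
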(event EventBeginPlay
  (Variables|Default|SetStartLocation (Transformation|GetWorldLocation (Variables|Default|GetPlateformStaticMesh)))
  (Utilities|FlowControl|Delay (Variables|Default|GetStartDelay))
  (Components|Timeline|SetPlayRate (Variables|Default|GetMove) (Variables|Default|GetSpeed))
  (bind _newtrack_0 (Timeline|Move PlayFromStart)
    (:Update
      (Transformation|SetWorldLocation (Variables|Default|GetPlateformStaticMesh) (+ (Variables|Default|GetStartLocation) (* _newtrack_0 (Variables|Default|GetVelocityImpulse))) false false))))

(fn ConstructionScript)