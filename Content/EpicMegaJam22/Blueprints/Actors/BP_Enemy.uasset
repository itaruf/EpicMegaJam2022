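; BP_Enemy is an enemy actor driven by a BP_EnemyController AI controller, made for EpicMegaJam22.
; On BeginPlay it caches that controller, then records its location as Start after a short delay, provided the controller cast succeeds.
; A custom Destroy event removes the actor after a brief delay.
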(event Custom|Destroy
  (Utilities|FlowControl|Delay 0.1)
  (Actor|DestroyActor))

(event EventBeginPlay
  (Utilities|FlowControl|Sequence
    (:then_0
      (bind _asbp_enemy_controller (Utilities|Casting|CastToBP_EnemyController (AI|GetAIController self)))
      (Variables|Default|Set%20BP%20Enemy%20Controller _asbp_enemy_controller))
    (:then_1
      (Utilities|FlowControl|Delay 0.2)
      (Variables|Default|SetStart (Transformation|GetActorLocation)))))

(fn ConstructionScript)