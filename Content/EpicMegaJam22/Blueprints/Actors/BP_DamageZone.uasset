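; BP_DamageZone is an actor that repeatedly damages the player while their BP_TwoWorldsCharacter overlaps it.
; Overlap start applies damage immediately through DamagePlayer and starts a looping timer at the DamageFrequence interval.
; DamagePlayer fetches the player through the MLGetPlayer macro rather than using the overlapping actor, then calls TakeDamage with DamageDone.
; Overlap end clears and invalidates the timer.
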(event Custom|DamagePlayer
  (bind _player (Utilities|MLGetPlayer)
    (:Out
      (Default|TakeDamage _player (Variables|Effects|GetDamageDone)))))

(event EventBeginPlay)

(event Collision|EventActorBeginOverlap
  (params (OtherActor :type Actor%20Object%20Reference))
  (Utilities|Casting|CastToBP_TwoWorldsCharacter OtherActor)
  (CallFunction|DamagePlayer)
  (bind _returnvalue (Utilities|Time|SetTimerbyEvent (EventDispatchers|CreateEvent :!event Custom|DamagePlayer) (Variables|Effects|GetDamageFrequence) true))
  (Variables|Effects|SetDamageTimer _returnvalue))

(event Collision|EventActorEndOverlap
  (params (OtherActor :type Actor%20Object%20Reference))
  (Utilities|Casting|CastToBP_TwoWorldsCharacter OtherActor)
  (Utilities|Time|ClearandInvalidateTimerbyHandle (Variables|Effects|GetDamageTimer)))

(fn ConstructionScript)