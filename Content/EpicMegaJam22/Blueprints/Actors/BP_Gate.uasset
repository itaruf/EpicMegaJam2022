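; BP_Gate is a gate actor that slides open and closed, and can be linked to an interactable trigger.
; On BeginPlay it binds an event to the interact dispatcher on AssociatedTrigger's BP_InteractionComponent, if present.
; TriggerDoor chooses Open or Close, which play or reverse a Speed-scaled timeline; its update moves Anchor along VelocityImpulse.
; A rotation-based timeline remains in the graph but never runs.
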(event Custom|Trigger%20Door
  (params (bool :type Boolean))
  (if bool
    (CallFunction|Open)
    (else
      (CallFunction|Close))))

(event Custom|Close
  (Components|Timeline|SetPlayRate (Variables|Default|GetTimeline_2) (Variables|Default|GetSpeed))
  (bind _newtrack_0 (Timeline|Timeline_2 Reverse)
    (:Update
      (Transformation|SetRelativeLocation (Variables|Default|GetAnchor) (* _newtrack_0 (Variables|Trigger|GetVelocityImpulse)) false false))))

(event Custom|Open
  (Components|Timeline|SetPlayRate (Variables|Default|GetTimeline_2) (Variables|Default|GetSpeed))
  (bind _newtrack_0 (Timeline|Timeline_2 Play)
    (:Update
      (Transformation|SetRelativeLocation (Variables|Default|GetAnchor) (* _newtrack_0 (Variables|Trigger|GetVelocityImpulse)) false false))))

(event EventBeginPlay
  (Utilities|FlowControl|Sequence
    (:then_0
      (Variables|Default|SetStartingRotation (Transformation|GetActorRotation))
      (Variables|Default|SetStartingPos (Transformation|GetActorLocation)))
    (:then_1
      (bind _associatedtrigger (Variables|Trigger|GetAssociatedTrigger)
        (:then
          (Utilities|IsValid (Actor|GetComponentbyClass _associatedtrigger "/Game/EpicMegaJam22/Blueprints/Actors/BP_InteractionComponent.BP_InteractionComponent_C")
            (:Is%20Valid
              (EventDispatchers|BindEventtoEDIonInteract (Actor|GetComponentbyClass _associatedtrigger "/Game/EpicMegaJam22/Blueprints/Actors/BP_InteractionComponent.BP_InteractionComponent_C") (EventDispatchers|CreateEvent :!event Custom|Trigger%20Door)))))
        (:else)))))

(fn ConstructionScript)