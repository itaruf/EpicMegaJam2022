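; Game mode for TwoWorlds that runs level flow: collectible goals, player death and level completion.
; On BeginPlay it binds to player death, HUD and item events, sets the level's item target and finds its ID in a map.
; Enough collected items fires a collect-finished dispatcher for the gate.
; End sequences show HUD widgets and fade out, then reload, advance or return to the opening screen; advice display is unwired.
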(event Custom|IsCollectFinished
  (params (NumberCollected :type Integer))
  ;[1 1 1] Check for if player has collected all the items to open the gate
  (if (>= NumberCollected (Variables|Default|GetNumToCollect))
    (Default|CallEDIonCollectFinished NumberCollected)))

(event Custom|SetHud
  ;[1 1 1] Hud set by event call
  (Variables|Default|SetPlayerHUD (HUD|GetHUD (Game|GetPlayerController 0))))

(event Custom|EndLevelSequence
  ;[1 1 1] End level (success) sequence
  (if (== (Variables|Default|GetCurrentLevelId) 4)
    (bind _asbp_two_worlds_hud (Utilities|Casting|CastToBP_TwoWorldsHud (Variables|Default|GetPlayerHUD)))
    (Default|DisplayEndGameWidget _asbp_two_worlds_hud (Variables|Default|GetFadeDuration))
    (Variables|Default|SetCurrentLevelId 0)
    (CameraFades|StartCameraFade (Game|GetPlayerCameraManager 0) 0.0 1.0 (Variables|Default|GetFadeDuration) "(R=1.000000,G=1.000000,B=1.000000,A=1.000000)" false true)
    (Utilities|FlowControl|Delay (Variables|Default|GetFadeDuration))
    (Game|OpenLevel(byName) "OpeningScreen")
    (else
      (bind _asbp_two_worlds_hud_2 (Utilities|Casting|CastToBP_TwoWorldsHud (Variables|Default|GetPlayerHUD)))
      (Default|DisplaySuccessWidget _asbp_two_worlds_hud_2 (Variables|Default|GetFadeDuration) 0.0)
      (CameraFades|StartCameraFade (Game|GetPlayerCameraManager 0) 0.0 1.0 (Variables|Default|GetFadeDuration) "(R=1.000000,G=1.000000,B=1.000000,A=1.000000)" false true)
      (Utilities|FlowControl|Delay (Variables|Default|GetFadeDuration))
      (bind _result (Math|Integer|IncrementInt (Variables|Default|GetCurrentLevelId))
        (:%20%20
          (if (.ReturnValue (Utilities|Map|Find (Variables|Default|GetMapIdLevels) _result))
            (Game|OpenLevel(byName) (Utilities|String|StringToName (.Value (Utilities|Map|Find (Variables|Default|GetMapIdLevels) _result))))
            (else
              (Game|OpenLevel(byName) "FirstLevel"))))))))

(event Custom|DisplayAdvice
  (params (Advice :type String))
  ;[1 1 1] Display an advice
)

(event Custom|StartDeathSequence
  ;[1 1 1] Player death
  (if (not (Variables|Default|GetDeathSequenceStarted))
    (Variables|Default|SetDeathSequenceStarted true)
    (bind _asbp_two_worlds_hud (Utilities|Casting|CastToBP_TwoWorldsHud (Variables|Default|GetPlayerHUD)))
    (Default|HideUI _asbp_two_worlds_hud)
    (Default|DisplayDeathWidget _asbp_two_worlds_hud (Variables|Default|GetFadeDuration))
    (CameraFades|StartCameraFade :self (Game|GetPlayerCameraManager 0) :ToAlpha 1.0 :Duration (Variables|Default|GetFadeDuration) :bHoldWhenFinished true)
    (Utilities|FlowControl|Delay (Variables|Default|GetFadeDuration))
    (bind _returnvalue (Game|GetCurrentLevelName true))
    (Game|OpenLevel(byName) (Utilities|String|StringToName _returnvalue))))

(event EventBeginPlay
  (Utilities|FlowControl|Sequence
    (:then_0
      (bind _asbp_two_worlds_character (Utilities|Casting|CastToBP_TwoWorldsCharacter (Game|Player|GetPlayerPawn 0)))
      (bind _output_get (Variables|Default|SetPlayer _asbp_two_worlds_character))
      (EventDispatchers|BindEventtoEDIonPlayerDeath _asbp_two_worlds_character (EventDispatchers|CreateEvent :!event Custom|StartDeathSequence))
      (EventDispatchers|BindEventtoEDIonHudSet _asbp_two_worlds_character (EventDispatchers|CreateEvent :!event Custom|SetHud))
      (EventDispatchers|BindEventtoEDIonCollectedItem _output_get (EventDispatchers|CreateEvent :!event Custom|IsCollectFinished)))
    (:then_1
      (bind _returnvalue (Game|GetCurrentLevelName true))
      (switch string _returnvalue
        (:Default
          (Variables|Default|SetNumToCollect 0))
        (:Level2
          (Variables|Default|SetNumToCollect 3))
        (:Level3
          (Variables|Default|SetNumToCollect 3 :!label _label))
        (:Level4
          (goto _label))))
    (:then_2
      ;[1 1 1] Finding the current level ID to use to open the next level
      (bind _returnvalue_2 (Game|GetCurrentLevelName true))
      (Variables|Default|SetCurrentLevelName _returnvalue_2)
      (bind _keys (Utilities|Map|Keys (Variables|Default|GetMapIdLevels)))
      (for _array_element _keys
        (if (and (Utilities|Enum|Equal(Enum) (.Value (Utilities|Map|Find (Variables|Default|GetMapIdLevels) _array_element)) (Variables|Default|GetCurrentLevelName)) (.ReturnValue (Utilities|Map|Find (Variables|Default|GetMapIdLevels) _array_element)))
          (Variables|Default|SetCurrentLevelId _array_element))))))

(fn ConstructionScript)